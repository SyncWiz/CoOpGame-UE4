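; BP_TargetDummy is a target dummy that visualizes point damage and ragdolls when hit by radial damage.
; Point damage draws a brief debug sphere and the damage number at the hit location.
; Radial damage enables physics simulation on the skeletal mesh, then applies a large velocity-change impulse opposite the impact normal with an added upward bias.
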(event Game|Damage|EventRadialDamage
  (params (DamageReceived :type Float%20%28single-precision%29) (DamageType :type Damage%20Type%20Object%20Reference) (Origin :type Vector :default "0, 0, 0") (HitInfo :type Hit%20Result%20Structure%20%28by%20ref%29) (InstigatedBy :type Controller%20Object%20Reference) (DamageCauser :type Actor%20Object%20Reference))
  (bind _skeletalmesh (Variables|Default|GetSkeletalMesh))
  (Physics|SetSimulatePhysics _skeletalmesh true)
  (Physics|AddImpulse _skeletalmesh (* (* (+ (.ImpactNormal (Collision|BreakHitResult HitInfo)) "0, 0,-1.000000") -1.0) 1e+04) "None" true))

(event Game|Damage|EventPointDamage
  (params (Damage :type Float%20%28single-precision%29) (DamageType :type Damage%20Type%20Object%20Reference) (HitLocation :type Vector :default "0, 0, 0") (HitNormal :type Vector :default "0, 0, 0") (HitComponent :type Primitive%20Component%20Object%20Reference) (BoneName :type Name :default "None") (ShotFromDirection :type Vector :default "0, 0, 0") (InstigatedBy :type Controller%20Object%20Reference) (DamageCauser :type Actor%20Object%20Reference) (HitInfo :type Hit%20Result%20Structure%20%28by%20ref%29))
  (Rendering|Debug|DrawDebugSphere HitLocation 5.0 12 "(R=1.000000,G=0.926708,B=0.050526,A=1.000000)" 1.0 1.0)
  (Rendering|Debug|DrawDebugString HitLocation (Utilities|String|ToString(Float) Damage) 0 "(R=1.000000,G=0.000000,B=0.017859,A=1.000000)" 1.0))

(fn ConstructionScript)